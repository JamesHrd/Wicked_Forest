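; Monster that roams the map, hunts the player and triggers a paused game-over screen when it gets close.
; Tick wanders it with delayed random turns, halving its XY position when out of bounds away from the player.
; It chases faster on a proximity-weighted random roll when enough orbs are collected and the light is on, or always at a higher orb count.
; Distance bands select delayed roar, growl or footstep sounds.
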(event EventTick
  (params (DeltaSeconds :type Float%20%28single-precision%29))
  (bind _returnvalue (Transformation|GetActorLocation))
  (bind _returnvalue_2 (Transformation|GetActorLocation))
  (bind _returnvalue_3 (Game|GetPlayerController 0))
  (bind _returnvalue_4 (Game|Player|GetPlayerPawn 0))
  (bind _returnvalue_5 (Transformation|GetActorLocation))
  (bind _returnvalue_6 (Transformation|GetActorLocation _returnvalue_4))
  (bind _returnvalue_7 (- _returnvalue_6 _returnvalue_5))
  (bind _returnvalue_8 (Math|Vector|VectorLength _returnvalue_7))
  (bind _returnvalue_9 (Math|Float|Clamp(Float) _returnvalue_8 0.0 1e+04))
  ;[1 1 1] Detect kill
  (if (<= _returnvalue_8 1.5e+02)
    ;[1 1 1] Controll death screen
    (bind _asnew_hud (Utilities|Casting|CastToNewHUD (HUD|GetHUD (Game|GetPlayerController 0))))
    (Default|GameOver (Variables|/Game/Blueprints/NewHUD.NewHUD_C|GetUI_Ref _asnew_hud))
    (Game|SetGamePaused true)
    (Variables|/Script/Engine.PlayerController|SetbShowMouseCursor _returnvalue_3 true)
    (Input|SetInputModeUIOnly _returnvalue_3 0 "DoNotLock")
    (Variables|/Script/Engine.PlayerController|SetbShowMouseCursor _returnvalue_3 true)
    (else
      ;[1 1 1] Control random movement or direct to player
      (if (not (or (and (<= (Math|Random|RandomFloatinRange 0.0 _returnvalue_9) 5e+01) (and (>= (Variables|/Game/MISC/Game_Instance_Main.Game_Instance_Main_C|GetOrbs_Collected (stale EventBeginPlay _asgame_instance_main)) 2.0) (Variables|/Game/MISC/Game_Instance_Main.Game_Instance_Main_C|GetLight_Enabled (stale EventBeginPlay _asgame_instance_main)))) (>= (Variables|/Game/MISC/Game_Instance_Main.Game_Instance_Main_C|GetOrbs_Collected (stale EventBeginPlay _asgame_instance_main)) 1e+01)))
        ;[1 1 1] Move forward
        (Transformation|AddLocalOffset (Variables|Default|GetDefaultSceneRoot) (Math|Vector|MakeVector (* (Utilities|Time|GetWorldDeltaSeconds) 3e+02) 0.0 0.0) false false)
        (if (and (Math|Boolean|ORBoolean (>= (.x _returnvalue) 3.1e+04) (<= (.x _returnvalue) -1.9e+04) (>= (.y _returnvalue) 2.2e+04) (<= (.y _returnvalue) -3e+04)) (not (<= _returnvalue_9 1e+03)))
          ;[1 1 1] Reset creature position due to o-o-b
          (Transformation|SetWorldLocation (Variables|Default|GetDefaultSceneRoot) (/ (Transformation|GetActorLocation) "2.000000,2.000000,1.000000") false false)
          (else
            ;[1 1 1] Rotate randomly
            (Utilities|FlowControl|Delay 1.0)
            (Transformation|AddWorldRotation (Variables|Default|GetDefaultSceneRoot) (Math|Rotator|MakeRotator 0.0 0.0 (Math|Random|RandomFloatinRange -45.0 45.0)) false false)))
        (else
          ;[1 1 1] Movement directly to player
          (Transformation|SetWorldRotation (Variables|Default|GetDefaultSceneRoot) (Math|Rotator|MakeRotator 0.0 0.0 (.yaw (Math|Rotator|FindLookatRotation (Transformation|GetActorLocation) (Transformation|GetActorLocation (Game|Player|GetPlayerPawn 0))))) false false)
          (Transformation|AddLocalOffset (Variables|Default|GetDefaultSceneRoot) (Math|Vector|MakeVector (* (Utilities|Time|GetWorldDeltaSeconds) 5e+02) 0.0 0.0) false false)))
      ;[1 1 1] Control noises
      (if (>= _returnvalue_8 5e+04)
        (Utilities|FlowControl|Delay (Math|Random|RandomFloatinRange 15.0 3e+01))
        (Audio|PlaySoundatLocation "/Game/MISC/Roar_Cue.Roar_Cue" _returnvalue_2 "0, 0, 0" 1.0 1.0 0.0 "/Game/MISC/C_Long_attenuation.C_Long_attenuation" 0 0 0)
        (elif (and (<= _returnvalue_8 4.9e+04) (>= _returnvalue_8 5e+03))
          (Utilities|FlowControl|Delay (Math|Random|RandomFloatinRange 5.0 15.0))
          (Audio|PlaySoundatLocation "/Game/MISC/Growl_Cue.Growl_Cue" _returnvalue_2 "0, 0, 0" 1.0 1.0 0.0 "/Game/MISC/C_Medium_attenuation.C_Medium_attenuation" 0 0 0)
          (elif (<= _returnvalue_8 1.5e+04)
            (Utilities|FlowControl|Delay 0.8)
            (Audio|PlaySoundatLocation "/Game/MISC/Step_Cue.Step_Cue" _returnvalue_2 "0, 0, 0" 1.0 1.0 0.0 "/Game/MISC/C_Short_attenuation.C_Short_attenuation" 0 0 0)))))))

(event EventBeginPlay
  ;[1 1 1] Control if creature hunts or not
  (bind _asgame_instance_main (Utilities|Casting|CastToGame_Instance_Main (Game|GetGameInstance))))

(fn ConstructionScript)