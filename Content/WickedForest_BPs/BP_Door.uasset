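; BP_Door is a door that opens once enough orbs are collected, and it also scatters those orbs across the map.
; BeginPlay spawns nine BP_Orb actors at random XY positions at a fixed height.
; Tick polls OrbsCollected on Game_Instance_Main and, at ten or more, snaps the two Cylinder components to mirrored open rotations without animation.
; The threshold is one higher than the number of orbs spawned here.
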(event EventBeginPlay
  (while (< (Variables|Default|GetSpawned) 9.0)
    (Game|SpawnActorfromClass "/Game/WickedForest_BPs/BP_Orb.BP_Orb_C" (Math|Transform|MakeTransform (Math|Vector|MakeVector (Math|Random|RandomFloatinRange -2e+04 3.1e+04) (Math|Random|RandomFloatinRange -3.2e+04 2.2e+04) 1e+02) "0, 0, 0" "1.000000,1.000000,1.000000") "AdjustIfPossibleButAlwaysSpawn" 0 0)
    (Math|Float|IncrementFloat (Variables|Default|GetSpawned))))

(event EventTick
  (params (DeltaSeconds :type Float%20%28single-precision%29))
  (bind _asgame_instance_main (Utilities|Casting|CastToGame_Instance_Main (Game|GetGameInstance)))
  (if (>= (Variables|/Game/MISC/Game_Instance_Main.Game_Instance_Main_C|GetOrbs_Collected _asgame_instance_main) 1e+01)
    (Transformation|SetRelativeRotation (Variables|Default|GetCylinder) "0,110.000000, 0" false false)
    (Transformation|SetRelativeRotation (Variables|Default|GetCylinder1) "0,-110.000000, 0" false false)))

(fn ConstructionScript)