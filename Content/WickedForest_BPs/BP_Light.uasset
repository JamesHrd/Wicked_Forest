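; BP_Light is the player's guide light, which either follows the camera or flies off to show the way to the next objective.
; Each Tick it reads Game_Instance_Main and destroys itself when LightEnabled is off.
; While Locating, it yaws and steps toward the nearest tagged BP_Orb, or toward a BP_Winning_Box once ten orbs are collected.
; Otherwise it copies the camera transform, swapping the NLocal and NGlobal particles per mode.
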(event EventTick
  (params (DeltaSeconds :type Float%20%28single-precision%29))
  (bind _returnvalue (Game|GetPlayerCameraManager 0))
  (bind _returnvalue_2 (Transformation|GetActorLocation))
  (bind _returnvalue_3 (Transformation|GetActorLocation _returnvalue))
  (bind _returnvalue_4 (Transformation|GetActorRotation _returnvalue))
  ;[1 1 1] Controls light enabled or destroyed
  (bind _asgame_instance_main (Utilities|Casting|CastToGame_Instance_Main (Game|GetGameInstance))
    (:then
      (if (Variables|/Game/MISC/Game_Instance_Main.Game_Instance_Main_C|GetLight_Enabled _asgame_instance_main)
        ;[1 1 1] Locating or Holding
        (if (Variables|/Game/MISC/Game_Instance_Main.Game_Instance_Main_C|GetLocating _asgame_instance_main)
          ;[1 1 1] Particles for locating
          (Components|Activation|SetActive (Variables|Default|GetN_Local) false false)
          (Components|Activation|SetActive (Variables|Default|GetN_Global) true false)
          ;[1 1 1] Target orbs or door
          (if (< (Variables|/Game/MISC/Game_Instance_Main.Game_Instance_Main_C|GetOrbs_Collected _asgame_instance_main) 1e+01)
            ;[1 1 1] Finds and moves to nearest Orb
            (bind _outactors (Actor|GetAllActorsOfClasswithTag "/Game/WickedForest_BPs/BP_Orb.BP_Orb_C" "Orb"))
            (Transformation|SetActorRotation (Math|Rotator|MakeRotator 0.0 0.0 (.yaw (Math|Rotator|FindLookatRotation _returnvalue_2 (Transformation|GetActorLocation (.ReturnValue (Actor|FindNearestActor _returnvalue_2 _outactors)))))))
            (Transformation|AddLocalOffset (Variables|Default|GetDefaultSceneRoot) "5.000000,0.000000, 0" false false)
            (else
              ;[1 1 1] Moves to the gate
              (bind _outactors_2 (Actor|GetAllActorsOfClass "/Game/WickedForest_BPs/BP_Winning_Box.BP_Winning_Box_C"))
              (Transformation|SetActorRotation (Math|Rotator|MakeRotator 0.0 0.0 (.yaw (Math|Rotator|FindLookatRotation (Transformation|GetActorLocation) (Transformation|GetActorLocation (.ReturnValue (Actor|FindNearestActor "0, 0, 0" _outactors_2)))))))
              (Transformation|AddLocalOffset (Variables|Default|GetDefaultSceneRoot) "5.000000,0.000000, 0" false false)))
          (else
            ;[1 1 1] Particles for holding
            (Components|Activation|SetActive (Variables|Default|GetN_Local) true false)
            (Components|Activation|SetActive (Variables|Default|GetN_Global) false false)
            ;[1 1 1] Attach light to player
            (Transformation|SetActorLocationAndRotation (Math|Vector|MakeVector (.x _returnvalue_3) (.y _returnvalue_3) (.z _returnvalue_3)) (Math|Rotator|MakeRotator (.roll _returnvalue_4) (.pitch _returnvalue_4) (.yaw _returnvalue_4)))))
        (else
          (Actor|DestroyActor))))
    (:CastFailed
      (Development|PrintString "Nope4"))))

(fn ConstructionScript)