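; BP_Orb is a collectible orb that adds to the game's collected orb count when overlapped.
; Any actor overlap increments OrbsCollected on Game_Instance_Main, with no check on which actor entered.
; It then refreshes the text through the UI reference on player zero's NewHUD and destroys itself, which only happens if that HUD cast succeeds.
; A failed game instance cast just prints a debug string.
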(event Collision|EventActorBeginOverlap
  (params (OtherActor :type Actor%20Object%20Reference))
  ;[1 1 1] Increments Orbs_Collected by 1
  (bind _asgame_instance_main (Utilities|Casting|CastToGame_Instance_Main (Game|GetGameInstance))
    (:then
      (Math|Float|IncrementFloat (Variables|/Game/MISC/Game_Instance_Main.Game_Instance_Main_C|GetOrbs_Collected _asgame_instance_main)
        (:%20%20
          ;[1 1 1] Update UI text
          (bind _asnew_hud (Utilities|Casting|CastToNewHUD (HUD|GetHUD (Game|GetPlayerController 0))))
          (Default|UpdateText (Variables|/Game/Blueprints/NewHUD.NewHUD_C|GetUI_Ref _asnew_hud))
          (Actor|DestroyActor))))
    (:CastFailed
      (Development|PrintString "Nope"))))

(fn ConstructionScript)